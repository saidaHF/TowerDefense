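; BP_GMB tracks the selected tile and recolors paper-sprite tiles for hover, selection and deselection.
; OnClickTileBP stores the current tile as the last one and, only if it is valid, deselects it and applies the selected color to the clicked tile.
; Deselection restores the base color when the sprite shows the selected color, while hover tints any tile except the current one.
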(fn `OnClickTileBP`
  (params (tileTarget :type "/Game/BP/TileBP Object Reference"))
  ;[0.6848 1 0.5705] deselect and select new
  (bind _output_get (set `self.lastTileBP` (`self.actualTileBP`)))
  (`/Engine/EditorBlueprintResources/StandardMacros.IsValid` _output_get
    (:`Is Valid`
      (`self.OnDeselectTileBP` _output_get)
      (bind _output_get_2 (set `self.actualTileBP` tileTarget))
      (`/Game/BP/TileBP.SetColor` _output_get_2 (`self.SelectedColor`)))))

(fn `OnDeselectTileBP`
  (params (TileTarget :type "/Game/BP/TileBP Object Reference"))
  (if (and (== null (`self.actualTileBP`)) (`KismetMathLibrary.LinearColor_IsNearEqual` (`PaperSpriteComponent.SpriteColor` (`/Game/BP/TileBP.PaperSprite` TileTarget)) (`self.SelectedColor`)))
    (`/Game/BP/TileBP.SetColor` TileTarget (`self.BaseColor`))))

(fn `OnHoverTileBP`
  (params (TileTarget :type "/Game/BP/TileBP Object Reference"))
  (if (not (== TileTarget (`self.actualTileBP`)))
    (`/Game/BP/TileBP.SetColor` TileTarget (`self.HoverColor`))))

(fn `UserConstructionScript`)